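; BP_Door is an interactable door that swings open and closed on its yaw axis.
; Each Interaction event alternates through a FlipFlop, playing an open or closing sound at the door and running the OpenDoor timeline forward or in reverse to lerp the rotation through a quarter turn.
; A Box overlap shows the Widget on entry and hides it on exit, with no check on which actor overlaps.
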(event `/Game/ThirdPerson/Blueprints/Interaction_Interface.Interaction`
  (bind _returnvalue (`SceneComponent.K2_GetComponentLocation` (`self.Door`)))
  (`/Engine/EditorBlueprintResources/StandardMacros.FlipFlop`
    (:`A`
      (`GameplayStatics.PlaySoundAtLocation` "/Game/SoundEffect/Open_Door.Open_Door" _returnvalue (struct) 1.0 1.0 0.0 null null null null)
      (bind (_direction _door) (`Timeline|Open Door` :!label _label)
        (:`Update`
          (`SceneComponent.K2_SetRelativeRotation` (`self.Door`) (`KismetMathLibrary.MakeRotator` 0.0 0.0 (`KismetMathLibrary.Lerp` 0.0 90.0 _door)) false false))))
    (:`B`
      (`GameplayStatics.PlaySoundAtLocation` "/Game/SoundEffect/Closing_Door.Closing_Door" _returnvalue (struct) 1.0 1.0 0.0 null null null null)
      (goto _label :!via `Reverse`))))

(event `self.Box.OnComponentBeginOverlap`
  (params (OverlappedComponent :type "PrimitiveComponent Object Reference") (OtherActor :type "Actor Object Reference") (OtherComp :type "PrimitiveComponent Object Reference") (OtherBodyIndex :type Integer) (bFromSweep :type Boolean) (SweepResult :type "HitResult Structure (by ref)"))
  (bind _output_get (set `self.Widget` (`self.Widget`)))
  (`SceneComponent.SetVisibility` _output_get true false))

(event `self.Box.OnComponentEndOverlap`
  (params (OverlappedComponent :type "PrimitiveComponent Object Reference") (OtherActor :type "Actor Object Reference") (OtherComp :type "PrimitiveComponent Object Reference") (OtherBodyIndex :type Integer))
  (bind _output_get (set `self.Widget` (`self.Widget`)))
  (`SceneComponent.SetVisibility` _output_get false false))

(fn `UserConstructionScript`)